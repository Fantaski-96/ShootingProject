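; BP_Player is the player-controlled shooter actor, moving in the Y-Z plane and firing bullets.
; BeginPlay adds the Enhanced Input mapping context, and horizontal and vertical input actions store their axis values.
; Tick normalizes those values and moves the actor by speed and delta time without sweeping for collisions.
; The fire action spawns BP_Bullet at the FirePosition component and plays a randomly pitched blaster sound.
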(event Input|EnhancedActionEvents|EnhancedInputActionIA_Horizontal
  (params (ActionValue :type Float%20%28double-precision%29) (ElapsedSeconds :type Float%20%28double-precision%29) (TriggeredSeconds :type Float%20%28double-precision%29) (InputAction :type Input%20Action%20Object%20Reference :default "/Game/Inputs/IA_Horizontal.IA_Horizontal"))
  ;[1 1 1] A, D 좌우 버튼
  (:Triggered
    (Variables|Default|SetHorizontal ActionValue))
  (:Completed
    (Variables|Default|SetHorizontal ActionValue)))

(event Input|EnhancedActionEvents|EnhancedInputActionIA_Vertical
  (params (ActionValue :type Float%20%28double-precision%29) (ElapsedSeconds :type Float%20%28double-precision%29) (TriggeredSeconds :type Float%20%28double-precision%29) (InputAction :type Input%20Action%20Object%20Reference :default "/Game/Inputs/IA_Vertical.IA_Vertical"))
  ;[1 1 1] W, S 앞뒤 버튼
  (:Triggered
    (Variables|Default|SetVertical ActionValue))
  (:Completed
    (Variables|Default|SetVertical ActionValue)))

(event Input|EnhancedActionEvents|EnhancedInputActionIA_Fire
  (params (ActionValue :type Boolean) (ElapsedSeconds :type Float%20%28double-precision%29) (TriggeredSeconds :type Float%20%28double-precision%29) (InputAction :type Input%20Action%20Object%20Reference :default "/Game/Inputs/IA_Fire.IA_Fire"))
  ;[1 1 1] Bullet
  (:Started
    (Game|SpawnActorfromClass "/Game/BluePrints/BP_Bullet.BP_Bullet_C" (Transformation|GetWorldTransform (Variables|Default|GetFire%20Position)) "AlwaysSpawn" "MultiplyWithRoot" 0 0)
    (Audio|PlaySound2D "/Game/Audio/star-wars-blaster.star-wars-blaster" 1.0 (Math|Random|RandomFloatinRange 1.0 3.0) 0.0 0 0)))

(event Input|EnhancedActionEvents|EnhancedInputActionIA_QuitGame
  (params (ActionValue :type Boolean) (ElapsedSeconds :type Float%20%28double-precision%29) (TriggeredSeconds :type Float%20%28double-precision%29) (InputAction :type Input%20Action%20Object%20Reference :default "/Game/Inputs/IA_QuitGame.IA_QuitGame")))

(event EventBeginPlay
  (Input|AddMappingContext (PlayerController|LocalPlayerSubsystems|GetEnhancedInputLocalPlayerSubsystem (Game|GetPlayerController 0)) "/Game/Inputs/IMC_PlayerInput.IMC_PlayerInput" 0 "(bIgnoreAllPressedKeysUntilRelease=True,bForceImmediately=False,bNotifyUserSettings=False)"))

(event EventTick
  (params (DeltaSeconds :type Float%20%28single-precision%29))
  ;[1 1 1] 이동 노드 BP
  (Transformation|SetActorLocation (+ (Transformation|GetActorLocation) (* (* (Math|Vector|Normalize (Math|Vector|MakeVector 0.0 (Variables|Default|GetHorizontal) (Variables|Default|GetVertical))) (Variables|Default|GetMoveSpeed)) DeltaSeconds)) false false))

(fn ConstructionScript)