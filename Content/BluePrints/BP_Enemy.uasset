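; Enemy actor that flies in a straight line and ends the game when it touches the player.
; On BeginPlay a random roll against TraceRate either aims it once at BP_Player's current location or keeps its forward vector.
; Tick moves it along that fixed direction at MoveSpeed without sweeping.
; Overlapping the player destroys the player, spawns an explosion, shows the game-over widget and cursor, and pauses the game.
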(event Collision|EventActorBeginOverlap
  (params (OtherActor :type Actor%20Object%20Reference))
  ;[1 1 1] 플레이어와 컨텍시 폭발
  (bind _asbp_player (Utilities|Casting|CastToBP_Player OtherActor))
  (Actor|DestroyActor _asbp_player)
  (Effects|SpawnEmitteratLocation "/Game/StarterContent/Particles/P_Explosion.P_Explosion" (Transformation|GetActorLocation))
  (bind _returnvalue (Game|ConstructObjectfromClass "/Game/UI/WBP_GameOverWidget.WBP_GameOverWidget_C"))
  (UserInterface|Viewport|AddtoViewport _returnvalue 0)
  (Variables|/Script/Engine.PlayerController|SetbShowMouseCursor (Game|GetPlayerController 0) true)
  (Game|SetGamePaused true))

(event EventTick
  (params (DeltaSeconds :type Float%20%28single-precision%29))
  ;[1 1 1] Enemy BP
  (Transformation|SetActorLocation (+ (Transformation|GetActorLocation) (* (* (Variables|Default|GetDierction) (Variables|Default|GetMoveSpeed)) DeltaSeconds)) false false))

(event EventBeginPlay
  ;[1 1 1] 랜덤 플레이어 추적 로직 BP
  (if (<= (Math|Random|RandomFloatinRange 0.0 1.0) (Variables|Default|GetTraceRate))
    (bind _returnvalue (Actor|GetActorOfClass "/Game/BluePrints/BP_Player.BP_Player_C"))
    (Utilities|IsValid _returnvalue
      (:Is%20Valid
        (bind _output_get (Variables|Default|SetDierction (Math|Vector|Normalize (- (Transformation|GetActorLocation _returnvalue) (Transformation|GetActorLocation)))))
        (Transformation|SetActorRotation (Math|Rotator|MakeRotfromXZ _output_get (Transformation|GetActorUpVector)))))
    (else
      (Variables|Default|SetDierction (Transformation|GetActorForwardVector)))))

(fn ConstructionScript)