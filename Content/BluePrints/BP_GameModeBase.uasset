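; BP_GameModeBase is the game mode that tracks the current score and a persistent best score.
; On BeginPlay it adds the main widget to the viewport and loads the saved best score.
; AddScore accumulates points and, whenever the current score beats the best, immediately writes it through a BP_SaveScore save object to the BestScoreData slot.
; Loading checks that the slot exists before reading it.
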(event EventBeginPlay
  (bind _returnvalue (UserInterface|CreateWidget "/Game/UI/WBP_MainWidget.WBP_MainWidget_C"))
  (UserInterface|Viewport|AddtoViewport _returnvalue 0)
  (bind _bestscore (CallFunction|LoadScoreData))
  (Variables|Default|SetBastScore _bestscore))

(fn ConstructionScript)

(fn AddScore
  (params (Point :type Integer))
  (bind _output_get (Variables|Default|SetCurrentScore (+ Point (Variables|Default|GetCurrentScore))))
  (if (> _output_get (Variables|Default|GetBastScore))
    (bind _output_get_2 (Variables|Default|SetBastScore _output_get))
    (CallFunction|SaveScoreData _output_get_2)))

(fn SaveScoreData
  (params (Save%20Value :type Integer))
  (bind _returnvalue (SaveGame|CreateSaveGameObject "/Game/BluePrints/BP_SaveScore.BP_SaveScore_C"))
  (bind _output_get (Variables|Default|SetSave%20Instance _returnvalue))
  (Variables|/Game/BluePrints/BP_SaveScore.BP_SaveScore_C|SetScoreData _output_get Save%20Value)
  (SaveGame|SaveGametoSlot _output_get "BestScoreData"))

(fn LoadScoreData
  ;[1 1 1] 저장된 데이터가 있는지 확인
  (bind _returnvalue (SaveGame|DoesSaveGameExist "BestScoreData"))
  (if _returnvalue
    (bind _returnvalue_2 (SaveGame|LoadGamefromSlot "BestScoreData"))
    (bind _asbp_save_score (Utilities|Casting|CastToBP_SaveScore _returnvalue_2))
    (return (Variables|/Game/BluePrints/BP_SaveScore.BP_SaveScore_C|GetScoreData _asbp_save_score))))